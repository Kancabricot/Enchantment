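; BP_PickUp_Overboard is a pickup actor that grants the overboard power to a third-person character and equips it.
; When its trigger overlaps a BP_ThirdPersonCharacter, it searches the mesh's child components for an existing BP_Overboard.
; If none is found, it sets the character's power enum, adds a BP_Overboard component with automatic attachment and destroys itself.
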(event OnComponentBeginOverlap(TriggerPickUp)
  (params (OverlappedComponent :type Primitive%20Component%20Object%20Reference) (OtherActor :type Actor%20Object%20Reference) (OtherComp :type Primitive%20Component%20Object%20Reference) (OtherBodyIndex :type Integer) (bFromSweep :type Boolean) (SweepResult :type Hit%20Result%20Structure%20%28by%20ref%29))
  ;[1 1 1] Give the power and equip it
  (bind _asbp_third_person_character (Utilities|Casting|CastToBP_ThirdPersonCharacter OtherActor))
  (bind _array_element (Utilities|Array|ForEachLoopwithBreak (Components|GetChildrenComponents (Variables|/Script/Engine.Character|GetMesh _asbp_third_person_character) false) :!label _label)
    (:LoopBody
      (Utilities|Casting|CastToBP_Overboard _array_element)
      (Variables|Default|SetbCharaterHasOverboard true)
      (goto _label Break))
    (:Completed
      (if (not (Variables|Default|GetbCharaterHasOverboard))
        (Variables|/Game/02-Blueprints/02-Player/BP_ThirdPersonCharacter.BP_ThirdPersonCharacter_C|SetEnum_Power _asbp_third_person_character "NewEnumerator1")
        (AddComponent|AddBPOverboard _asbp_third_person_character false)
        (Actor|DestroyActor)))))

(fn ConstructionScript)